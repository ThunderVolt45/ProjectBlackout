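; Breakable pillar actor that swaps its intact static mesh for physics-simulated debris pieces.
; The BreakPillartest event hides the main mesh and disables its collision, then reveals each child actor tagged BreakPiece with query-only collision and physics enabled.
; Unconnected leftover logic would rebuild the pillar by hiding the pieces and restoring WholeMeshRef, or re-break it after a delay, but never runs.
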(event Custom|BreakPillartest
  (bind _returnvalue (Actor|GetComponentbyClass "/Script/Engine.StaticMeshComponent"))
  (Development|SetHiddeninGame _returnvalue true false)
  (Rendering|SetVisibility _returnvalue false false)
  (Collision|SetCollisionEnabled _returnvalue "NoCollision")
  (for _array_element (Actor|GetComponentsByClass "/Script/Engine.ChildActorComponent")
    (if (Components|ComponentHasTag _array_element "BreakPiece")
      (Development|PrintString "Hello")
      (Development|SetHiddeninGame (Actor|GetComponentbyClass (Variables|/Script/Engine.ChildActorComponent|GetChildActor _array_element) "/Script/Engine.StaticMeshComponent") false false)
      (Rendering|SetVisibility (Actor|GetComponentbyClass (Variables|/Script/Engine.ChildActorComponent|GetChildActor _array_element) "/Script/Engine.StaticMeshComponent") true false)
      (Collision|SetCollisionEnabled (Actor|GetComponentbyClass (Variables|/Script/Engine.ChildActorComponent|GetChildActor _array_element) "/Script/Engine.StaticMeshComponent") "QueryOnly")
      (Physics|SetSimulatePhysics (Actor|GetComponentbyClass (Variables|/Script/Engine.ChildActorComponent|GetChildActor _array_element) "/Script/Engine.StaticMeshComponent") true))))

(event EventBeginPlay)

(fn ConstructionScript)